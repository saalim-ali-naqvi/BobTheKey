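; BP_key is a key pickup in the BobTheCoin game that grants a key to the player.
; It overrides the parent's PickedThisUp event, calls the parent, then casts the picking actor to BP_MainCharecter and passes its KeyType to GetAKey.
; The BeginPlay, overlap and Tick events are disabled stubs, and the construction script only calls the parent.
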(event `self.PickedThisUp`
  (params (ActorThatPickedThisUp :type "Actor Object Reference"))
  (`parent.PickedThisUp` ActorThatPickedThisUp)
  (bind _asbp_main_charecter (cast `/Game/BobTheCoin/Core/Player/BP_MainCharecter` ActorThatPickedThisUp))
  (`/Game/BobTheCoin/Core/Player/BP_MainCharecter.GetAKey` _asbp_main_charecter (`self.KeyType`)))

(fn `UserConstructionScript`
  (`parent.UserConstructionScript`))