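; Game mode for BobTheCoin that tracks the player's respawn point and handles winning.
; On BeginPlay it takes the PlayerStart transform as the initial respawn point.
; UpdateRespawnPoint resets the previous checkpoint via ReturnToNormal, then stores the new transform and checkpoint reference.
; WinTheGame prints a win message and triggers the main character's celebration.
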(event `self.ReceiveBeginPlay`
  (bind _returnvalue (`GameplayStatics.GetActorOfClass` "/Script/Engine.PlayerStart"))
  (set `self.Respawnpoint` (`self.GetTransform` _returnvalue)))

(event `WinTheGame`
  (`KismetSystemLibrary.PrintString` "You Won!")
  (bind _asbp_main_charecter (cast `/Game/BobTheCoin/Core/Player/BP_MainCharecter` (`GameplayStatics.GetPlayerCharacter` 0)))
  (`/Game/BobTheCoin/Core/Player/BP_MainCharecter.EnterCelebration` _asbp_main_charecter))

(fn `UpdateRespawnPoint`
  (params (NewRespawnpoint :type "Transform Structure") (CheckpointRef :type "/Game/BobTheCoin/Core/RespawnSystem/BP_CheckPoint Object Reference"))
  (bind _currentcheckpoint_ref (`self.CurrentCheckpoint Ref`))
  (`|ExecutionSequence`
    (:`then_0`
      (if (`KismetSystemLibrary.IsValid` _currentcheckpoint_ref)
        (`/Game/BobTheCoin/Core/RespawnSystem/BP_CheckPoint.ReturnToNormal` _currentcheckpoint_ref)))
    (:`then_1`
      (set `self.Respawnpoint` (`local.NewRespawnpoint`))
      (set `self.CurrentCheckpoint Ref` (`local.CheckpointRef`)))))

(fn `UserConstructionScript`)